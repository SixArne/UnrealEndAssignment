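; BP_Flag is a flag actor that starts a chase once it is collected.
; On BeginPlay it binds to the OnFlagCollected delegate, and a FlagIsCollected guard makes the response run only once.
; That response plays the theme sound in 2D and spawns a BP_Chaser at SpawnPosition, which the construction script caches from the Billboard component's world location.
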(event Custom|FlagCollected
  (if (not (Variables|Default|GetFlagIsCollected))
    (Variables|Default|SetFlagIsCollected true)
    (Audio|PlaySound2D "/Game/Audio/CUE_Theme.CUE_Theme" 1.0 1.0 0.0 0 0)
    (Game|SpawnActorfromClass "/Game/Blueprints/BP_Chaser.BP_Chaser_C" (Math|Transform|MakeTransform (Variables|Default|GetSpawnPosition) "0, 0, 0" "1,1,1") "Undefined" 0 0)))

(event EventBeginPlay
  (EventDispatchers|BindEventtoOnFlagCollectedDelegate (delegate Custom|FlagCollected)))

(event EventTick
  (params (DeltaSeconds :type Float%20%28single-precision%29)))

(fn ConstructionScript
  (Variables|Default|SetSpawnPosition (Transformation|GetWorldLocation (Variables|Default|GetBillboard))))