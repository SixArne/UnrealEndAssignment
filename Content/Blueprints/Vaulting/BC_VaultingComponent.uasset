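; Actor component that lets a BP_Character vault onto ledges in front of it.
; While idle, it line-traces downward ahead each tick, checks ledge height, slope and capsule clearance, and shows or hides the WI_Vault prompt.
; The Vault event starts a state in which Tick teleports the owner along a lerp to the cached landing point.
; Debug traces, capsules and prints are left enabled.
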(event Custom|Vault
  ;[1 1 1] Vault event
  (Variables|Private|SetProgress 0.0)
  (Variables|Private|SetStartingLocation (Transformation|GetActorLocation (Variables|Private|GetOwningCharacter)))
  (Variables|Private|SetVaultingState "NewEnumerator2")
  (Development|PrintString (Utilities|String|ToString(Vector) (Variables|Public|GetEnding%20Location)) true true "(R=0.904232,G=0.000000,B=1.000000,A=1.000000)"))

(event EventBeginPlay
  ;[1 1 1] Cache owner and create Widget to display later
  (bind _asbp_character (Utilities|Casting|CastToBP_Character (Components|GetOwner)))
  (Variables|Private|SetOwningCharacter _asbp_character)
  (bind _returnvalue (UserInterface|CreateWidget "/Game/Blueprints/Vaulting/WI_Vault.WI_Vault_C" (.AsPlayer%20Controller (Utilities|Casting|CastToPlayerController (Pawn|GetController (Variables|Private|GetOwningCharacter))))))
  (Variables|Private|SetVaultWidget _returnvalue))

(event EventTick
  (params (DeltaSeconds :type Float%20%28single-precision%29))
  (Utilities|SwitchVaultingState
    (:NotVaulting
      ;[1 1 1] If not vaulting check if can vault and add/remove ui element
      (bind (_result _endinglocation) (Public|CanVault))
      (if _result
        (Variables|Public|SetEnding%20Location _endinglocation)
        ;;[1 1 1] Add to screen
        (if (not (UserInterface|Viewport|IsinViewport (Variables|Private|GetVaultWidget)))
          (UserInterface|Viewport|AddtoViewport (Variables|Private|GetVaultWidget) 0))
        (else
          ;;[1 1 1] Remove from screen if on screen
          (if (UserInterface|Viewport|IsinViewport (Variables|Private|GetVaultWidget))
            (Widget|RemovefromParent (Variables|Private|GetVaultWidget))))))
    (:Vaulting
      (Private|TickVault DeltaSeconds))))

(fn CanVault
  (bind _owningcharacter (Variables|Private|GetOwningCharacter))
  (bind _vaultdistance (Variables|Default|GetVaultDistance))
  (bind _returnvalue (Transformation|GetActorLocation _owningcharacter))
  (bind _returnvalue_2 (Transformation|GetActorForwardVector _owningcharacter))
  (bind _returnvalue_3 (* _returnvalue_2 _vaultdistance))
  (bind _returnvalue_4 (+ _returnvalue _returnvalue_3))
  (if (Utilities|Enum|Equal(Enum) (Variables|Private|GetVaultingState) "NewEnumerator0")
    (LocalVariables|SetCapsule%20%28local%29 (Variables|/Script/Engine.Character|GetCapsuleComponent (Variables|Private|GetOwningCharacter)))
    (bind (_outhit _returnvalue_5) (Collision|LineTraceByChannel (+ _returnvalue_4 (Math|Vector|MakeVector 0.0 0.0 (Components|Capsule|GetScaledCapsuleHalfHeight (LocalVariables|GetCapsule%20%28local%29)))) (- _returnvalue_4 (Math|Vector|MakeVector 0.0 0.0 (Components|Capsule|GetScaledCapsuleHalfHeight (LocalVariables|GetCapsule%20%28local%29)))) "TraceTypeQuery1" false (Utilities|Array|MakeArray (Variables|Private|GetOwningCharacter)) "ForOneFrame"))
    (if _returnvalue_5
      (bind (_result _endinglocation) (Private|CanVaulttoHit _outhit (LocalVariables|GetCapsule%20%28local%29)))
      (return _result _endinglocation)
      (else
        (return false "0, 0, 0")))
    (else
      (return false "0, 0, 0"))))

(fn CanVaulttoHit
  (params (HitResult :type Hit%20Result%20Structure) (PlayerCapsule :type Capsule%20Component%20Object%20Reference))
  (bind _z (Math|Vector|BreakVector (.location HitResult)))
  (bind _returnvalue (Components|Capsule|GetScaledCapsuleRadius PlayerCapsule))
  (bind _z_2 (Math|Vector|BreakVector (.traceend HitResult)))
  (bind _returnvalue_2 (- _z _z_2))
  (Utilities|FlowControl|Sequence
    (:then_0
      ;[1 1 1] Make sure that ledge is at an appropriate height
      (Development|PrintString (Utilities|String|ToString(Float) _returnvalue_2) true true "(R=0.107088,G=1.000000,B=0.000000,A=1.000000)" 0.0)
      (if (not (Math|Float|InRange(Float) _returnvalue_2 (Variables|Private|Constants|GetMinVaultingHeight) (Variables|Private|Constants|GetMaxVaultingHeight)))
        (return false "0, 0, 0")))
    (:then_1
      ;[1 1 1] Make sure its not slanted
      (if (< (.Z (Math|Vector|BreakVector (.normal HitResult))) (Class|CharacterMovementComponent|GetWalkableFloorZ (Variables|/Script/Engine.Character|GetCharacterMovement (Variables|Private|GetOwningCharacter))))
        (return false "0, 0, 0")))
    (:then_2
      ;[1 1 1] Make sure that there is enough room on top of the ledge
      (bind _output_get (LocalVariables|SetEndingLocation%20%28local%29 (+ (.location HitResult) (Math|Vector|MakeVector 0.0 0.0 (Components|Capsule|GetScaledCapsuleHalfHeight PlayerCapsule)))))
      (bind _result (Private|CheckCapsuleCollision (+ _output_get (Math|Vector|MakeVector 0.0 0.0 _returnvalue)) (Components|Capsule|GetScaledCapsuleHalfHeight PlayerCapsule) _returnvalue true))
      (if _result
        (return false "0, 0, 0")))
    (:then_3
      ;[1 1 1] Return when all other checks succeeded
      (return true (LocalVariables|GetEndingLocation%20%28local%29)))))

(fn CheckCapsuleCollision
  (params (Center :type Vector) (HalfHeight :type Float%20%28single-precision%29) (Radius :type Float%20%28single-precision%29) (DrawDebug :type Boolean))
  (Utilities|FlowControl|Sequence
    (:then_0
      (if DrawDebug
        (Rendering|Debug|DrawDebugCapsule Center HalfHeight Radius "0, 0, 0" "(R=1.000000,G=0.846547,B=0.000000,A=1.000000)" 0.0 3.0)))
    (:then_1
      (bind _returnvalue (Collision|CapsuleOverlapActors Center Radius HalfHeight (Utilities|Array|MakeArray "ObjectTypeQuery1" "ObjectTypeQuery2" "ObjectTypeQuery4" "ObjectTypeQuery5" "ObjectTypeQuery6") "/Script/Engine.Actor" (Utilities|Array|MakeArray (Variables|Private|GetOwningCharacter))))
      (return _returnvalue))))

(fn TickVault
  (params (DeltaSeconds :type Float%20%28single-precision%29))
  (Utilities|FlowControl|Sequence
    (:then_0
      (Variables|Private|SetProgress (Math|Float|Clamp(Float) (+ DeltaSeconds (/ (Variables|Private|GetProgress) (Variables|Private|Constants|GetVaultSpeed)))))
      (Transformation|SetActorLocation (Variables|Private|GetOwningCharacter) (Math|Vector|Lerp(Vector) (Variables|Private|GetStartingLocation) (Variables|Public|GetEnding%20Location) (Variables|Private|GetProgress)) false true))
    (:then_1
      (if (>= (Variables|Private|GetProgress) 1.0)
        (Variables|Private|SetVaultingState "NewEnumerator0")))))