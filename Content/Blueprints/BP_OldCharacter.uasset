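; BP_OldCharacter is a character Blueprint that adds smoothed crouching and sprinting.
; BeginPlay caches capsule half height and max speed as baselines for Timeline-driven lerps, which reverse when each action ends.
; OnStartCrouch lerps capsule height toward HalfHeightAdjust, while the StartCrouch/StopCrouch pair, marked deprecated, targets CrouchedHalfHeight.
; Running lerps MaxWalkSpeed toward MaxSpeed and plays a camera shake until it stops.
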(event Custom|StartCrouch
  ;[1 1 1] DEPRECATED
  (Variables|Default|SetIsCrouching true)
  (bind _lerpvalue (Timeline|CrouchSmoothing Play)
    (:Update
      (Components|Capsule|SetCapsuleHalfHeight (Variables|Collision|GetCapsuleComponent) (Math|Float|Lerp (Variables|Default|GetCapsuleHalfHeight) (Variables|/Script/Engine.CharacterMovementComponent|GetCrouchedHalfHeight (Variables|Character|GetCharacterMovement)) _lerpvalue) true))))

(event Custom|StopCrouch
  ;[1 1 1] DEPRECATED
  (Variables|Default|SetIsCrouching false)
  (bind _lerpvalue (Timeline|CrouchSmoothing Reverse)
    (:Update
      (Components|Capsule|SetCapsuleHalfHeight (Variables|Collision|GetCapsuleComponent) (Math|Float|Lerp (Variables|Default|GetCapsuleHalfHeight) (Variables|/Script/Engine.CharacterMovementComponent|GetCrouchedHalfHeight (Variables|Character|GetCharacterMovement)) _lerpvalue) true))))

(event Custom|OnStartRunning
  ;[0.03666 0.228 0.7396] Run smoothing
  (Variables|Default|SetIsRunning true)
  (bind _returnvalue (CameraShakes|StartCameraShake (Game|GetPlayerCameraManager 0) "/Game/Blueprints/BP_CameraShake.BP_CameraShake_C" 1.0 "CameraLocal" "0, 0, 0"))
  (Variables|Default|SetSprintCameraShakeRef _returnvalue)
  (bind _lerpvalue (Timeline|SmoothRunning Play)
    (:Update
      (Variables|/Script/Engine.CharacterMovementComponent|SetMaxWalkSpeed (Variables|Character|GetCharacterMovement) (Math|Float|Lerp (Variables|Default|GetNormalSpeed) (Variables|Default|GetMaxSpeed) _lerpvalue)))))

(event Custom|OnEndRunning
  ;[0.03666 0.228 0.7396] Run smoothing
  (Variables|Default|SetIsRunning false)
  (CameraShakes|StopCameraShake (Game|GetPlayerCameraManager 0) (Variables|Default|GetSprintCameraShakeRef) false)
  (bind _lerpvalue (Timeline|SmoothRunning Reverse)
    (:Update
      (Variables|/Script/Engine.CharacterMovementComponent|SetMaxWalkSpeed (Variables|Character|GetCharacterMovement) (Math|Float|Lerp (Variables|Default|GetNormalSpeed) (Variables|Default|GetMaxSpeed) _lerpvalue)))))

(event EventOnEndCrouch
  (params (HalfHeightAdjust :type Float%20%28single-precision%29) (ScaledHalfHeightAdjust :type Float%20%28single-precision%29))
  ;[1 1 1] Crouch smoothing
  (bind _lerpvalue (Timeline|SmoothCrouching Reverse)
    (:Update
      (Components|Capsule|SetCapsuleHalfHeight (Variables|Collision|GetCapsuleComponent) (Math|Float|Lerp (Variables|Default|GetCapsuleHalfHeight) (stale EventOnStartCrouch HalfHeightAdjust) _lerpvalue) true))))

(event EventBeginPlay
  ;[1 1 1] Set original half height
  (Variables|Default|SetCapsuleHalfHeight (Variables|/Script/Engine.CapsuleComponent|GetCapsuleHalfHeight (Variables|Collision|GetCapsuleComponent)))
  ;[1 1 1] Cache max speed
  (Variables|Default|SetNormalSpeed (Class|MovementComponent|GetMaxSpeed (Variables|Character|GetCharacterMovement))))

(event EventOnStartCrouch
  (params (HalfHeightAdjust :type Float%20%28single-precision%29) (ScaledHalfHeightAdjust :type Float%20%28single-precision%29))
  ;[1 1 1] Crouch smoothing
  (bind _lerpvalue (Timeline|SmoothCrouching Play)
    (:Update
      (Components|Capsule|SetCapsuleHalfHeight (Variables|Collision|GetCapsuleComponent) (Math|Float|Lerp (Variables|Default|GetCapsuleHalfHeight) HalfHeightAdjust _lerpvalue) true))))

(fn ConstructionScript)