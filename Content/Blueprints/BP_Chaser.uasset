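; BP_Chaser is an actor that continuously moves toward the player character.
; On BeginPlay it finds and caches the BP_Character instance as its target.
; Each Tick it offsets itself along the normalized direction to that target, scaled by MoveSpeed and delta time, teleporting without sweep so collisions do not block it.
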(event EventBeginPlay
  (bind _returnvalue (Actor|GetActorOfClass "/Game/Blueprints/BP_Character.BP_Character_C"))
  (Variables|Default|SetPlayer _returnvalue))

(event EventTick
  (params (DeltaSeconds :type Float%20%28single-precision%29))
  (Transformation|AddActorWorldOffset (* (* (Math|Vector|Normalize (- (Transformation|GetActorLocation (Variables|Default|GetPlayer)) (Transformation|GetActorLocation))) (Variables|Default|GetMoveSpeed)) DeltaSeconds) false true))

(fn ConstructionScript)