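; BP_StartSound is a trigger volume that plays a 2D sound when a BP_Character enters it.
; The box's begin-overlap event casts the other actor to BP_Character, then plays Cue and sets IsPlaying.
; IsPlaying is never reset in these graphs, so the sound starts only once.
; The construction script sizes the box from the Extent variable.
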(event OnComponentBeginOverlap(Box)
  (params (OverlappedComponent :type Primitive%20Component%20Object%20Reference) (OtherActor :type Actor%20Object%20Reference) (OtherComp :type Primitive%20Component%20Object%20Reference) (OtherBodyIndex :type Integer) (bFromSweep :type Boolean) (SweepResult :type Hit%20Result%20Structure%20%28by%20ref%29))
  (Utilities|Casting|CastToBP_Character OtherActor)
  (if (not (Variables|Default|GetIsPlaying))
    (Audio|PlaySound2D (Variables|Settings|GetCue) 1.0 1.0 0.0 0 0)
    (Variables|Default|SetIsPlaying true)))

(event EventBeginPlay)

(fn ConstructionScript
  (Components|Box|SetBoxExtent (Variables|Default|GetBox) (Variables|Settings|GetExtent) true))