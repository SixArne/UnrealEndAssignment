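; BP_ResetZone is a trigger volume actor that teleports the player character back to a reset point.
; On BeginPlay it caches the ResetPoint component's world location as the spawn point.
; When a BP_Character overlaps the Box, it is moved there with a teleport and no sweep.
; The construction script sizes the Box from the Extent variable.
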(event OnComponentBeginOverlap(Box)
  (params (OverlappedComponent :type Primitive%20Component%20Object%20Reference) (OtherActor :type Actor%20Object%20Reference) (OtherComp :type Primitive%20Component%20Object%20Reference) (OtherBodyIndex :type Integer) (bFromSweep :type Boolean) (SweepResult :type Hit%20Result%20Structure%20%28by%20ref%29))
  (bind _asbp_character (Utilities|Casting|CastToBP_Character OtherActor))
  (Transformation|SetActorLocation _asbp_character (Variables|Default|GetSpawnpoint) false true))

(event EventBeginPlay
  (Variables|Default|SetSpawnpoint (Transformation|GetWorldLocation (Variables|Default|GetResetPoint))))

(event Collision|EventActorBeginOverlap
  (params (OtherActor :type Actor%20Object%20Reference)))

(event EventTick
  (params (DeltaSeconds :type Float%20%28single-precision%29)))

(fn ConstructionScript
  (Components|Box|SetBoxExtent (Variables|Default|GetBox) (Variables|Default|GetExtent) false))