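; BP_HintText is a world-placed hint that shows configurable text as the player character approaches.
; Overlap of a BP_Character with the box collider plays a timeline that scales the text's X and Y up, and leaving reverses it.
; Text starts at zero scale unless AlwaysVisible is set, and every tick it turns to face the player character's location, not the camera.
; The construction script applies the box extent and text.
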(event OnComponentBeginOverlap(Collider)
  (params (OverlappedComponent :type Primitive%20Component%20Object%20Reference) (OtherActor :type Actor%20Object%20Reference) (OtherComp :type Primitive%20Component%20Object%20Reference) (OtherBodyIndex :type Integer) (bFromSweep :type Boolean) (SweepResult :type Hit%20Result%20Structure%20%28by%20ref%29))
  (bind _textrender (Variables|Default|GetTextRender))
  ;[1 1 1] Fade in event button
  (Utilities|Casting|CastToBP_Character OtherActor)
  (bind _lerp (Timeline|Fade%20in Play)
    (:Update
      (Rendering|Components|TextRender|SetXScale _textrender _lerp)
      (Rendering|Components|TextRender|SetYScale _textrender _lerp))))

(event OnComponentEndOverlap(Collider)
  (params (OverlappedComponent :type Primitive%20Component%20Object%20Reference) (OtherActor :type Actor%20Object%20Reference) (OtherComp :type Primitive%20Component%20Object%20Reference) (OtherBodyIndex :type Integer))
  (bind _textrender (Variables|Default|GetTextRender))
  ;[1 1 1] Fade in event button
  (Utilities|Casting|CastToBP_Character OtherActor)
  (bind _lerp (Timeline|Fade%20in Reverse)
    (:Update
      (Rendering|Components|TextRender|SetXScale _textrender _lerp)
      (Rendering|Components|TextRender|SetYScale _textrender _lerp))))

(event EventBeginPlay
  (bind _textrender (Variables|Default|GetTextRender))
  ;[1 1 1] Set scale of icon to 0
  (if (not (Variables|Default|GetAlwaysVisible))
    (Rendering|Components|TextRender|SetXScale _textrender 0.0)
    (Rendering|Components|TextRender|SetYScale _textrender 0.0)))

(event EventTick
  (params (DeltaSeconds :type Float%20%28single-precision%29))
  ;[1 1 1] Rotate to camera
  (Transformation|SetWorldRotation (Variables|Default|GetTextRender) (Math|Rotator|FindLookatRotation (Transformation|GetWorldLocation (Variables|Default|GetTextRender)) (Transformation|GetActorLocation (Game|GetPlayerCharacter 0))) false false))

(fn ConstructionScript
  (Components|Box|SetBoxExtent (Variables|Default|GetCollider) (Variables|Settings|GetBox%20Extent) true)
  (Rendering|Components|TextRender|SetText (Variables|Default|GetTextRender) (Variables|Default|GetText)))