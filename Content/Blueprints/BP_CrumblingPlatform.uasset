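; A platform that crumbles after the player steps on it and later restores itself.
; A box overlap with BP_Character starts a timer that Tick advances.
; Past the crumble time, the mesh switches on physics and gravity to fall.
; At the reset time, it teleports back to the transform saved at BeginPlay, disables physics and clears the timer for reuse.
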(event OnComponentBeginOverlap(Box)
  (params (OverlappedComponent :type Primitive%20Component%20Object%20Reference) (OtherActor :type Actor%20Object%20Reference) (OtherComp :type Primitive%20Component%20Object%20Reference) (OtherBodyIndex :type Integer) (bFromSweep :type Boolean) (SweepResult :type Hit%20Result%20Structure%20%28by%20ref%29))
  (Utilities|Casting|CastToBP_Character OtherActor)
  (Variables|Default|SetPlayerHasTouchedPlatform true))

(event EventTick
  (params (DeltaSeconds :type Float%20%28single-precision%29))
  (bind _staticmesh (Variables|Default|GetStaticMesh))
  (if (Variables|Default|GetPlayerHasTouchedPlatform)
    (Variables|Default|SetCurrentTime (+ DeltaSeconds (Variables|Default|GetCurrentTime)))
    (Utilities|FlowControl|Sequence
      (:then_0
        (if (>= (Variables|Default|GetCurrentTime) (Variables|Default|GetTimeUntilCrumble))
          (Variables|Default|SetIsCrumbled true)
          (Physics|SetSimulatePhysics (Variables|Default|GetStaticMesh) true)
          (Physics|SetEnableGravity (Variables|Default|GetStaticMesh) true)))
      (:then_1
        (if (>= (Variables|Default|GetCurrentTime) (Variables|Default|GetResetTime))
          (Transformation|SetWorldLocation (Variables|Default|GetStaticMesh) (Variables|Default|GetOriginalPosition) false true)
          (Transformation|SetRelativeRotation (Variables|Default|GetStaticMesh) (Variables|Default|GetOriginalRotation) false false)
          (Physics|SetSimulatePhysics _staticmesh false)
          (Physics|SetEnableGravity _staticmesh false)
          (Variables|Default|SetPlayerHasTouchedPlatform false)
          (Variables|Default|SetIsCrumbled false)
          (Variables|Default|SetCurrentTime 0.0))))))

(event EventBeginPlay
  (Variables|Default|SetOriginalPosition (Transformation|GetWorldLocation (Variables|Default|GetStaticMesh)))
  (Variables|Default|SetOriginalRotation (Variables|/Script/Engine.SceneComponent|GetRelativeRotation (Variables|Default|GetStaticMesh))))

(fn ConstructionScript)